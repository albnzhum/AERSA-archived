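; Vostok1 is an interaction object that shows a prompt widget while the first-person character is near it.
; Box overlaps toggle CanInteract and the widget's visibility, and releasing F runs the same player check and hide logic as leaving the box.
; A non-looping timer yaws the widget toward the player once, a second after BeginPlay.
; NoIncr, YesIncr and WGActive are stubs returning false, and nothing here reads CanInteract.
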(event OnComponentBeginOverlap(Box)
  (params (OverlappedComponent :type Primitive%20Component%20Object%20Reference) (OtherActor :type Actor%20Object%20Reference) (OtherComp :type Primitive%20Component%20Object%20Reference) (OtherBodyIndex :type Integer) (bFromSweep :type Boolean) (SweepResult :type Hit%20Result%20Structure%20%28by%20ref%29))
  (if (== OtherActor (Variables|Default|GetAs%20First%20Person%20Character))
    (Variables|Default|SetCan%20interact true)
    (Rendering|SetVisibility (Variables|Default|GetWidget) true false)))

(event OnComponentEndOverlap(Box)
  (params (OverlappedComponent :type Primitive%20Component%20Object%20Reference) (OtherActor :type Actor%20Object%20Reference) (OtherComp :type Primitive%20Component%20Object%20Reference) (OtherBodyIndex :type Integer))
  (if (== (Variables|Default|GetAs%20First%20Person%20Character) OtherActor)
    (Variables|Default|SetCan%20interact false)
    (Rendering|SetVisibility (Variables|Default|GetWidget) false false)))

(event Custom|Spin
  (bind _widget (Variables|Default|GetWidget))
  (Transformation|SetWorldRotation _widget (Math|Rotator|MakeRotator 0.0 0.0 (.yaw (Math|Rotator|FindLookatRotation (Transformation|GetWorldLocation _widget) (Transformation|GetWorldLocation (Variables|/Script/Engine.Actor|GetRootComponent (Variables|Default|GetAs%20First%20Person%20Character)))))) false false))

(event EventBeginPlay
  (Utilities|FlowControl|Sequence
    (:then_0
      (bind _asfirst_person_character (Utilities|Casting|CastToFirstPersonCharacter (Game|GetPlayerCharacter 0)))
      (Variables|Default|SetAs%20First%20Person%20Character _asfirst_person_character)
      (Rendering|SetVisibility (Variables|Default|GetWidget) false false))
    (:then_1
      (Utilities|Time|SetTimerbyEvent (delegate Custom|Spin) 1.0))))

(event Collision|EventActorBeginOverlap
  (params (OtherActor :type Actor%20Object%20Reference)))

(event EventTick
  (params (DeltaSeconds :type Float%20%28single-precision%29)))

(event Input|KeyboardEvents|F
  (params (Key :type Key%20Structure :default "None"))
  (:Released
    (if (== (Variables|Default|GetAs%20First%20Person%20Character) (stale OnComponentEndOverlap(Box) OtherActor))
      (Variables|Default|SetCan%20interact false)
      (Rendering|SetVisibility (Variables|Default|GetWidget) false false))))

(fn ConstructionScript)

(fn NoIncr
  (return false))

(fn WGActive
  (return false))

(fn YesIncr
  (return false))